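; Behavior tree service that classifies how far the AI's controlled pawn is from its TargetToFollow actor.
; Each tick it writes the target's position to the TargetLocation blackboard key and measures the straight-line distance to it.
; Four threshold variables split that distance into non-overlapping melee, close, mid, far and too-far bands, each written to its own blackboard bool.
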(event `self.ReceiveTick`
  (params (OwnerActor :type "Actor Object Reference") (DeltaSeconds :type "Float (single-precision)"))
  (bind _toofardistance (`self.TooFarDistance`))
  (bind _middistance (`self.MidDistance`))
  (bind _fardistance (`self.FarDistance`))
  (bind _closedistance (`self.CloseDistance`))
  (bind _returnvalue (`Actor.K2_GetActorLocation` (`BTFunctionLibrary.GetBlackboardValueAsActor` (`self.TargetToFollow`))))
  (bind _returnvalue_2 (`KismetMathLibrary.VSize` (- _returnvalue (`Actor.K2_GetActorLocation` (`Controller.K2_GetPawn` (`self.AIRef`))))))
  (bind _asaicontroller (cast `AIController` OwnerActor))
  (set `self.AIRef` _asaicontroller)
  (`BTFunctionLibrary.SetBlackboardValueAsVector` (`self.TargetLocation`) _returnvalue)
  (`BTFunctionLibrary.SetBlackboardValueAsBool` (`self.IsAtMelee`) (< _returnvalue_2 _closedistance))
  (`BTFunctionLibrary.SetBlackboardValueAsBool` (`self.IsAtClose`) (and (>= _returnvalue_2 _closedistance) (< _returnvalue_2 _middistance)))
  (`BTFunctionLibrary.SetBlackboardValueAsBool` (`self.IsAtMid`) (and (>= _returnvalue_2 _middistance) (< _returnvalue_2 _fardistance)))
  (`BTFunctionLibrary.SetBlackboardValueAsBool` (`self.IsAtFar`) (and (>= _returnvalue_2 _fardistance) (< _returnvalue_2 _toofardistance)))
  (`BTFunctionLibrary.SetBlackboardValueAsBool` (`self.IsAtTooFar`) (>= _returnvalue_2 _toofardistance)))