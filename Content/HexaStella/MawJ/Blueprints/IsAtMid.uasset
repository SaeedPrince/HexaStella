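; Behavior tree decorator for the boss AI that checks whether the target to follow is at mid range.
; It casts its owner to Boss_Controller and measures the distance from the controlled pawn to the actor in the TargetToFollow blackboard key.
; The condition passes when that distance is at least MidBot and below MidTop, also printing an on-screen debug message.
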(fn `PerformConditionCheck`
  (params (OwnerActor :type "Actor Object Reference"))
  (returns (ReturnValue :type Boolean))
  (bind _returnvalue (`KismetMathLibrary.VSize` (- (`Actor.K2_GetActorLocation` (`BTFunctionLibrary.GetBlackboardValueAsActor` (`self.TargetToFollow`))) (`Actor.K2_GetActorLocation` (`Controller.K2_GetPawn` (`self.AIRef`))))))
  (bind _returnvalue_2 (and (< _returnvalue (`self.MidTop`)) (>= _returnvalue (`self.MidBot`))))
  (bind _asboss_controller (cast `/Game/HexaStella/MawJ/Blueprints/Boss_Controller` OwnerActor))
  (set `self.AIRef` _asboss_controller)
  (if _returnvalue_2
    (`KismetSystemLibrary.PrintString` "Target Is Mid" true false)
    (return _returnvalue_2)))