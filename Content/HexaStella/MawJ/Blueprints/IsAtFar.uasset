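; Behavior tree decorator for the boss AI that checks whether its follow target is far away.
; It casts the owner to Boss_Controller and measures the distance from the controlled pawn to the actor in the TargetToFollow blackboard key.
; The condition passes when that distance is at least FarDistance, printing a debug message to screen.
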(fn `PerformConditionCheck`
  (params (OwnerActor :type "Actor Object Reference"))
  (returns (ReturnValue :type Boolean))
  (bind _returnvalue (>= (`KismetMathLibrary.VSize` (- (`Actor.K2_GetActorLocation` (`BTFunctionLibrary.GetBlackboardValueAsActor` (`self.TargetToFollow`))) (`Actor.K2_GetActorLocation` (`Controller.K2_GetPawn` (`self.AIRef`))))) (`self.FarDistance`)))
  (bind _asboss_controller (cast `/Game/HexaStella/MawJ/Blueprints/Boss_Controller` OwnerActor))
  (set `self.AIRef` _asboss_controller)
  (if _returnvalue
    (`KismetSystemLibrary.PrintString` "Target Is Far" true false)
    (return _returnvalue)))