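; DamageTaken is a condition check for a boss AI that decides whether recent damage is high enough to trigger a block.
; It casts the owner to Boss_Controller and its controlled pawn to AI_Character, storing that pawn as AIRef.
; The check passes when the pawn's damage over the last three seconds exceeds EnoughToBlock and the controller reports its block is ready.
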(fn `PerformConditionCheck`
  (params (OwnerActor :type "Actor Object Reference"))
  (returns (ReturnValue :type Boolean))
  (bind _asboss_controller (cast `/Game/HexaStella/MawJ/Blueprints/Boss_Controller` OwnerActor))
  (`/Engine/EditorBlueprintResources/StandardMacros.IsValid` _asboss_controller
    (:`Is Valid`
      (bind _asai_character (cast `/Game/HexaStella/MawJ/Blueprints/AI_Character` (`Controller.K2_GetPawn` _asboss_controller)))
      (`/Engine/EditorBlueprintResources/StandardMacros.IsValid` _asai_character
        (:`Is Valid`
          (bind _output_get (set `self.AIRef` _asai_character))
          (return (and (> (`/Game/HexaStella/MawJ/Blueprints/AI_Character.DamagePerLastThreeSeconds` _output_get) (`self.EnoughToBlock`)) (`/Game/HexaStella/MawJ/Blueprints/Boss_Controller.BlockIsReady` _asboss_controller))))))))