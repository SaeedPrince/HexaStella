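; AI boss character that senses targets and tracks how much health it has recently lost.
; PawnSensing sight and hearing events pass the detected pawn or noise instigator to Boss_Controller as its target.
; Tick shifts health through four rolling snapshots to compute DamagePerLastThreeSeconds.
; The rounded timer check fires at about half a second, so the window is shorter than the name suggests.
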(event `self.PawnSensing.OnSeePawn`
  (params (Pawn :type "Pawn Object Reference"))
  ;[1 1 1] Target Detection
  (bind _asboss_controller (cast `/Game/HexaStella/MawJ/Blueprints/Boss_Controller` (`self.GetController`)))
  (`/Engine/EditorBlueprintResources/StandardMacros.IsValid` _asboss_controller
    (:`Is Valid`
      (`/Game/HexaStella/MawJ/Blueprints/Boss_Controller.SetTarget` _asboss_controller Pawn))))

(event `self.ReceiveBeginPlay`
  ;[1 1 1] Initialization
  (bind _output_get (set `self.Health` (`self.BaseHealth`)))
  (bind _output_get_2 (set `self.FirstHP` _output_get))
  (bind _output_get_3 (set `self.SecondHP` _output_get_2))
  (bind _output_get_4 (set `self.ThirdHP` _output_get_3))
  (set `self.FourthHP` _output_get_4))

(event `self.PawnSensing.OnHearNoise`
  (params (Instigator :type "Pawn Object Reference") (Location :type "Vector Structure (by ref)") (Volume :type "Float (single-precision)"))
  ;[1 1 1] Target Detection
  (bind _asboss_controller (cast `/Game/HexaStella/MawJ/Blueprints/Boss_Controller` (`self.GetController`)))
  (`/Engine/EditorBlueprintResources/StandardMacros.IsValid` _asboss_controller
    (:`Is Valid`
      (`/Game/HexaStella/MawJ/Blueprints/Boss_Controller.SetTarget` _asboss_controller Instigator))))

(event `self.ReceiveTick`
  (params (DeltaSeconds :type "Float (single-precision)"))
  ;[1 1 1] DamagePerLastThreeSeconds
  (bind _output_get (set `self.DeltaSecond` (+ (`self.DeltaSecond`) DeltaSeconds)))
  (if (== (`KismetMathLibrary.Conv_IntToDouble` (`KismetMathLibrary.Round` _output_get)) 1.0)
    (set `self.DeltaSecond` 0.0)
    (set `self.DamagePerLastThreeSeconds` (+ (- (`self.FourthHP`) (`self.Health`)) (- (`self.ThirdHP`) (`self.FourthHP`)) (- (`self.SecondHP`) (`self.ThirdHP`))))
    (set `self.FirstHP` (`self.SecondHP`))
    (set `self.SecondHP` (`self.ThirdHP`))
    (set `self.ThirdHP` (`self.FourthHP`))
    (set `self.FourthHP` (`self.Health`))))

(fn `UserConstructionScript`)