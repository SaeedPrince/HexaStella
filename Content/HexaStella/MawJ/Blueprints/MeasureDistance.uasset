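; A behavior tree node Blueprint that measures the distance between the boss and its target.
; It overrides PerformDistanceCheck, casting the owner to Boss_Controller to reach the controlled pawn.
; It returns the length of the vector between that pawn and the actor stored in the TargetToFollow blackboard key.
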(fn `PerformDistanceCheck`
  (params (OwnerActor :type "Actor Object Reference"))
  (returns (Distance :type "Float (double-precision)"))
  (bind _asboss_controller (cast `/Game/HexaStella/MawJ/Blueprints/Boss_Controller` OwnerActor))
  (set `self.AI_Controller` _asboss_controller)
  (return (`KismetMathLibrary.VSize` (- (`Actor.K2_GetActorLocation` (`BTFunctionLibrary.GetBlackboardValueAsActor` (`self.TargetToFollow`))) (`Actor.K2_GetActorLocation` (`Controller.K2_GetPawn` (`self.AI_Controller`)))))))