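; IsAtMelee is a Behavior Tree decorator that checks whether the boss's target is within melee range.
; It casts the owner to Boss_Controller and measures the distance from its controlled pawn to the TargetToFollow actor from the Blackboard.
; It passes when that distance is below MeleeDistance, also printing an on-screen debug message.
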(fn `PerformConditionCheck`
  (params (OwnerActor :type "Actor Object Reference"))
  (returns (ReturnValue :type Boolean))
  (bind _returnvalue (< (`KismetMathLibrary.VSize` (- (`Actor.K2_GetActorLocation` (`BTFunctionLibrary.GetBlackboardValueAsActor` (`self.TargetToFollow`))) (`Actor.K2_GetActorLocation` (`Controller.K2_GetPawn` (`self.AIRef`))))) (`self.MeleeDistance`)))
  (bind _asboss_controller (cast `/Game/HexaStella/MawJ/Blueprints/Boss_Controller` OwnerActor))
  (set `self.AIRef` _asboss_controller)
  (if _returnvalue
    (`KismetSystemLibrary.PrintString` "Target Is Melee" true false)
    (return _returnvalue)))